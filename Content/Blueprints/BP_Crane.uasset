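; BP_Crane is a crane actor that moves horizontally with a looping-style movement sound attached to its Cube component.
; SetXSpeed and SetYSpeed store axis inputs, and Tick offsets the actor location by them, scaled by MoveSpeed and delta time, without sweeping.
; UpdateSpeed tracks IsMoving against a small dead zone, switching the sound's volume multiplier on state changes rather than restarting the audio.
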(event EventBeginPlay
  (bind _returnvalue (Audio|SpawnSoundAttached (Variables|Default|GetSoundOfMoving) (Variables|Default|GetCube) "None" "0, 0, 0" "0, 0, 0" "KeepRelativeOffset" false 0.0 1.0 0.0 0 0))
  (Variables|Default|SetSound _returnvalue))

(event EventTick
  (params (DeltaSeconds :type Float%20%28single-precision%29))
  (CallFunction|UpdateLocation DeltaSeconds))

(fn ConstructionScript)

(fn UpdateLocation
  (params (DeltaSeconds :type Float%20%28single-precision%29))
  (bind _movespeed (Variables|Default|GetMoveSpeed))
  (Transformation|SetActorLocation (+ (Transformation|GetActorLocation) (Math|Vector|MakeVector (* DeltaSeconds (Variables|Default|GetXSpeed) _movespeed) (* DeltaSeconds (Variables|Default|GetYSpeed) _movespeed) 0.0)) false false))

(fn SetXSpeed
  (params (XSpeed :type Float%20%28single-precision%29))
  (Variables|Default|SetXSpeed XSpeed)
  (CallFunction|UpdateSpeed))

(fn SetYSpeed
  (params (YSpeed :type Float%20%28single-precision%29))
  (Variables|Default|SetYSpeed YSpeed)
  (CallFunction|UpdateSpeed))

(fn UpdateSpeed
  (bind _sound (Variables|Default|GetSound))
  (if (or (> (Math|Float|Absolute(Float) (Variables|Default|GetXSpeed)) 0.05) (> (Math|Float|Absolute(Float) (Variables|Default|GetYSpeed)) 0.05))
    (if (not (Variables|Default|GetIsMoving))
      (Variables|Default|SetIsMoving true)
      (Audio|Components|Audio|SetVolumeMultiplier _sound 1.0 :!class /Script/Engine.AudioComponent))
    (elif (Variables|Default|GetIsMoving)
      (Variables|Default|SetIsMoving false)
      (Audio|Components|Audio|SetVolumeMultiplier _sound 0.0 :!class /Script/Engine.AudioComponent))))