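; Player character Blueprint that grabs physics objects and operates levers and buttons with the left mouse button.
; Pressing traces a short line from the follow camera, grabs the hit component with a Physics Handle, then casts the actor to start holding a BP_LeverBox or push a BP_Button.
; Tick moves the handle target to the GrabLocation component.
; Releasing drops the component and lets go of any stored lever.
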(event Custom|PickUp
  (bind _followcamera (Variables|Default|GetFollowCamera))
  (bind _returnvalue (Transformation|GetWorldLocation _followcamera))
  (bind _returnvalue_2 (+ _returnvalue "0, 0,-10.000000"))
  (bind (_outhit _returnvalue_3) (Collision|LineTraceForObjects _returnvalue_2 (+ _returnvalue_2 (* (Math|Vector|GetForwardVector _followcamera) 5e+02)) (Utilities|Array|MakeArray "ObjectTypeQuery2" "ObjectTypeQuery4") false 0 "None"))
  (if _returnvalue_3
    (Variables|Default|SetPhysicsObject (.HitComponent (Collision|BreakHitResult _outhit)))
    (Class|PhysicsHandleComponent|GrabComponentatLocation (Variables|Default|GetPhysicsHandle) (.HitComponent (Collision|BreakHitResult _outhit)) "None" (.Location (Collision|BreakHitResult _outhit)))
    (bind _asbp_lever_box (Utilities|Casting|CastToBP_LeverBox (.HitActor (Collision|BreakHitResult _outhit)))
      (:then
        (bind _output_get (Variables|Default|SetLeverBox _asbp_lever_box))
        (Default|HoldLever _output_get true))
      (:CastFailed
        (bind _asbp_button (Utilities|Casting|CastToBP_Button (.HitActor (Collision|BreakHitResult _outhit))))
        (Default|PushButton _asbp_button)))))

(event Custom|Drop
  (bind _leverbox (Variables|Default|GetLeverBox))
  (Physics|Components|PhysicsHandle|ReleaseComponent (Variables|Default|GetPhysicsHandle))
  (Utilities|IsValid _leverbox
    (:Is%20Valid
      (Default|HoldLever _leverbox false))))

(event EventTick
  (params (DeltaSeconds :type Float%20%28single-precision%29))
  (Physics|Components|PhysicsHandle|SetTargetLocation (Variables|Default|GetPhysicsHandle) (Transformation|GetWorldLocation (Variables|Default|GetGrabLocation))))

(event Input|MouseEvents|LeftMouseButton
  (params (Key :type Key%20Structure :default "None"))
  (:Pressed
    (CallFunction|PickUp))
  (:Released
    (CallFunction|Drop)))

(fn ConstructionScript)