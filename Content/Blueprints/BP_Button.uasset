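; BP_Button is a pushable button that makes BP_Crane drop the sound block it holds.
; PushButton ignores presses while the button is already pushed, otherwise plays a sound and calls ReactOnPush, while Tick lerps the button's Z back up.
; ReactOnPush finds the crane, detaches any held block with physics enabled, runs its destroy check and deactivates BP_Grid's sound.
; A one-second timer then teleports the crane to its starting point.
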(event EventBeginPlay)

(event Collision|EventActorBeginOverlap
  (params (OtherActor :type Actor%20Object%20Reference)))

(event EventTick
  (params (DeltaSeconds :type Float%20%28single-precision%29))
  (if (Variables|Default|GetIsButtonPushed)
    (bind _output_get (Variables|Default|SetElapsedTime (+ DeltaSeconds (Variables|Default|GetElapsedTime))))
    (Transformation|SetRelativeLocation (Variables|Default|GetButton) (Math|Vector|MakeVector 0.0 0.0 (Math|Float|Lerp -8.0 0.0 (/ _output_get (Variables|Default|GetTimeToReturn)))) false false)
    (if (> (Variables|Default|GetElapsedTime) (Variables|Default|GetTimeToReturn))
      (Variables|Default|SetIsButtonPushed false))))

(fn ConstructionScript)

(fn PushButton
  (if (not (Variables|Default|GetIsButtonPushed))
    (Variables|Default|SetIsButtonPushed true)
    (Variables|Default|SetElapsedTime 0.0)
    (Audio|PlaySoundatLocation "/Game/Sound/button.button" (Transformation|GetActorLocation) "0, 0, 0" 1.0 1.0 0.0 0 0 0)
    (CallFunction|ReactonPush)))

(fn ReactonPush
  (bind _returnvalue (Actor|GetActorOfClass "/Game/Blueprints/BP_Crane.BP_Crane_C"))
  (LocalVariables|SetCrane _returnvalue)
  (Utilities|IsValid (Variables|/Game/Blueprints/BP_Crane.BP_Crane_C|GetCurrentSoundBlock _returnvalue)
    (:Is%20Valid
      (bind _asbp_sound_block (Utilities|Casting|CastToBP_SoundBlock (Variables|/Game/Blueprints/BP_Crane.BP_Crane_C|GetCurrentSoundBlock _returnvalue)))
      (Transformation|DetachFromActor _asbp_sound_block "KeepWorld" "KeepRelative" "KeepRelative")
      (Physics|SetSimulatePhysics (Variables|/Game/Blueprints/BP_SoundBlock.BP_SoundBlock_C|GetCube _asbp_sound_block) true)
      (Variables|/Game/Blueprints/BP_Crane.BP_Crane_C|SetCurrentSoundBlock (LocalVariables|GetCrane) 0)
      (Default|CheckDestroy _asbp_sound_block)
      (Utilities|Time|SetTimerbyFunctionName 0 "ReturnCrane" 1.0)
      (bind _returnvalue_2 (Actor|GetActorOfClass "/Game/Blueprints/BP_Grid.BP_Grid_C"))
      (Default|DeactivateSound _returnvalue_2))))

(fn ReturnCrane
  (bind _returnvalue (Actor|GetActorOfClass "/Game/Blueprints/BP_Crane.BP_Crane_C"))
  (Transformation|SetActorLocation _returnvalue (Variables|/Game/Blueprints/BP_Crane.BP_Crane_C|GetStartingPoint _returnvalue) false true)
  (Development|PrintString (Utilities|String|ToString(Vector) (Variables|/Game/Blueprints/BP_Crane.BP_Crane_C|GetStartingPoint _returnvalue))))