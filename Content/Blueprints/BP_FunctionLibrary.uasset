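; BP_FunctionLibrary is a Blueprint function library whose StopVelocityFn halts the physics motion of a given actor, with special handling for BP_Crane.
; It zeroes the linear velocity of all the actor's static mesh and cable components.
; For a crane, it switches off physics simulation on the Cone before the reset and back on afterwards.
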(fn StopVelocityFn
  (params (Actor :type Actor%20Object%20Reference))
  (bind _asbp_crane (Utilities|Casting|CastToBP_Crane Actor)
    (:then
      (bind _output_get (LocalVariables|SetCrane _asbp_crane))
      (Physics|SetSimulatePhysics (Variables|/Game/Blueprints/BP_Crane.BP_Crane_C|GetCone _output_get) false))
    (:CastFailed
      _))
  (for _array_element (Actor|GetComponentsByClass Actor "/Script/Engine.StaticMeshComponent")
    (Physics|SetPhysicsLinearVelocity _array_element "0, 0, 0" false "None"))
  (for _array_element_2 (Actor|GetComponentsByClass Actor "/Script/CableComponent.CableComponent")
    (Physics|SetPhysicsLinearVelocity _array_element_2 "0, 0, 0" false "None"))
  (Physics|SetSimulatePhysics (Variables|/Game/Blueprints/BP_Crane.BP_Crane_C|GetCone (LocalVariables|GetCrane)) true)
  (return))