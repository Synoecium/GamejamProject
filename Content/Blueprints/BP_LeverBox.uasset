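; BP_LeverBox is a lever control box that drives a crane's horizontal X and Y movement.
; Every tick it converts two lever rotations into actor-local space, scaling left-right roll into X speed and forward-back pitch into Y speed, both sign-inverted.
; HoldLever records whether a lever is held and tells the crane to correct its position on release.
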(event EventBeginPlay)

(event Collision|EventActorBeginOverlap
  (params (OtherActor :type Actor%20Object%20Reference)))

(event EventTick
  (params (DeltaSeconds :type Float%20%28single-precision%29))
  (Default|SetXSpeed (Variables|Default|GetCrane) (/ (.roll (Math|Transform|InverseTransformRotation (Transformation|GetActorTransform) (Transformation|GetWorldRotation (Variables|Default|GetLeverLR)))) -32.0))
  (Default|SetYSpeed (Variables|Default|GetCrane) (/ (.pitch (Math|Transform|InverseTransformRotation (Transformation|GetActorTransform) (Transformation|GetWorldRotation (Variables|Default|GetLeverFB)))) -32.0)))

(fn ConstructionScript)

(fn HoldLever
  (params (IsHold :type Boolean))
  (bind _output_get (Variables|Default|SetIsLeverHold IsHold))
  (if _output_get
    _
    (else
      (Default|CorrectPosition (Variables|Default|GetCrane))))
  (return))