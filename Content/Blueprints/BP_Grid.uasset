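; Grid actor that plays a sound when a BP_SoundBlock enters one of its cells.
; The construction script builds SizeX by SizeY box triggers, maps each to its coordinates and resizes an enclosing Box to fit.
; The cell's X index picks the sound, which replaces the current one unless it is the same sound.
; A helper returns an overlapped cell's location, and a crane ending overlap prints a debug message.
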(event EventBeginPlay)

(event Collision|EventActorBeginOverlap
  (params (OtherActor :type Actor%20Object%20Reference)))

(event EventTick
  (params (DeltaSeconds :type Float%20%28single-precision%29)))

(event Collision|EventActorEndOverlap
  (params (OtherActor :type Actor%20Object%20Reference))
  (Utilities|Casting|CastToBP_Crane OtherActor)
  (Development|PrintString "Beyaond!"))

(fn ConstructionScript
  (bind _box (Variables|Default|GetBox))
  (bind _sizex (Variables|Default|GetSizeX))
  (bind _sizey (Variables|Default|GetSizeY))
  (bind _returnvalue (- _sizex 1))
  (bind _returnvalue_2 (- _sizey 1))
  (for _index (range 1 (Variables|Default|GetSizeX))
    (for _index_2 (range 1 (Variables|Default|GetSizeY))
      (bind _returnvalue_3 (AddComponent|AddBoxComponent false (Math|Transform|MakeTransform (Math|Vector|MakeVector (* (- _index 1) 1.5e+02) (* (- _index_2 1) 1.5e+02) 0.0) "0, 0, 0" "1,1,2.000000")))
      (Utilities|Map|Add (Variables|Default|GetGridCoords) _returnvalue_3 (Utilities|Struct|MakeIntPoint (- _index 1) (- _index_2 1)))
      (Collision|BindEventtoOnComponentBeginOverlap _returnvalue_3 (EventDispatchers|CreateEvent :!event BPGridAutoGenFunc))
      (Transformation|SetRelativeScale3D _box (Math|Vector|MakeVector (+ (* _returnvalue 2.35) 1.5) (+ (* _returnvalue_2 2.35) 1.5) 1e+01))
      (Transformation|SetRelativeLocation _box (Math|Vector|MakeVector (* _returnvalue 75.0) (* _returnvalue_2 75.0) 2e+02) false false))))

(fn BPGridAutoGenFunc
  (params (OverlappedComponent :type Primitive%20Component%20Object%20Reference) (OtherActor :type Actor%20Object%20Reference) (OtherComp :type Primitive%20Component%20Object%20Reference) (OtherBodyIndex :type Integer) (bFromSweep :type Boolean) (SweepResult :type Hit%20Result%20Structure%20%28by%20ref%29))
  (LocalVariables|SetSoundBlock OtherActor)
  (if (== (Utilities|GetClass OtherActor) "/Game/Blueprints/BP_SoundBlock.BP_SoundBlock_C")
    (CallFunction|PlaySound (Utilities|Array|Get(acopy) (Variables|Default|GetSounds) (.x (.Value (Utilities|Map|Find (Variables|Default|GetGridCoords) OverlappedComponent)))) (Transformation|GetActorLocation OtherActor))
    (return)))

(fn PlaySound
  (params (Sound :type Sound%20Base%20Object%20Reference) (Location :type Vector))
  (if (Utilities|IsValid (Variables|Default|GetCurrentPlayingSound))
    (if (not (== (Variables|/Script/Engine.AudioComponent|GetSound (Variables|Default|GetCurrentPlayingSound)) Sound))
      (Components|Activation|SetActive (Variables|Default|GetCurrentPlayingSound) false false)
      (bind _returnvalue (Audio|SpawnSoundatLocation Sound Location "0, 0, 0" 1.0 1.0 0.0 0 0 :!label _label))
      (Variables|Default|SetCurrentPlayingSound _returnvalue))
    (else
      (goto _label))))

(fn IsActorOverlapsComponent
  (params (Actor :type Actor%20Object%20Reference))
  (bind _keys (Utilities|Map|Keys (Variables|Default|GetGridCoords)))
  (for _array_element _keys
    (if (Collision|IsOverlappingActor _array_element Actor :!class /Script/Engine.PrimitiveComponent)
      (return true (Transformation|GetWorldLocation _array_element))))
  (return false "0, 0, 0"))