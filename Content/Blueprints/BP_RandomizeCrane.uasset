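; BP_RandomizeCrane is a trigger actor that moves a BP_Crane to a random column of the grid when the crane overlaps it.
; It caches the level's BP_Grid on BeginPlay.
; On overlap, it picks a random column within the grid's SizeX and converts it to world X from the grid's bounds, keeping Y and Z.
; A debug print shows a separately rolled X, which can differ from the applied one.
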(event EventBeginPlay
  (bind _returnvalue (Actor|GetActorOfClass "/Game/Blueprints/BP_Grid.BP_Grid_C"))
  (Variables|Default|SetGrid _returnvalue))

(event Collision|EventActorBeginOverlap
  (params (OtherActor :type Actor%20Object%20Reference))
  (bind _grid (Variables|Default|GetGrid))
  (bind (_origin _boxextent) (Collision|GetActorBounds _grid false false))
  (bind _sizex (Variables|/Game/Blueprints/BP_Grid.BP_Grid_C|GetSizeX _grid))
  (bind _returnvalue (Math|Random|RandomInteger _sizex))
  (bind _returnvalue_2 (- (.x _origin) (.x _boxextent)))
  (bind _returnvalue_3 (* _returnvalue 1.5e+02))
  (bind _returnvalue_4 (+ _returnvalue_3 _returnvalue_2 5e+01))
  (bind _asbp_crane (Utilities|Casting|CastToBP_Crane OtherActor))
  (Transformation|SetActorLocation _asbp_crane (Math|Vector|MakeVector _returnvalue_4 (.y (Transformation|GetActorLocation _asbp_crane)) (.z (Transformation|GetActorLocation _asbp_crane))) false false)
  (Development|PrintString (Utilities|String|ToString(Float) _returnvalue_4) true true "(R=0.000000,G=0.660000,B=1.000000,A=1.000000)" 5.0))

(fn ConstructionScript)